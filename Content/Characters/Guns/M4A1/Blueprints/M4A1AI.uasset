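; M4A1AI is an M4A1 gun Blueprint, apparently an AI variant, with automatic hitscan fire and a toggleable laser.
; StartShooting loops Shoot on a timer, and StopShooting clears it and stops the player's camera shake.
; Shoot spawns a Niagara muzzle flash, calls a sound and applies point damage along a trace from player 0's mouse position, not the gun.
; The ammo check and decrement are disconnected, so shots consume no ammo.
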(event `self.ReceiveBeginPlay`
  (`parent.ReceiveBeginPlay`))

(event `self.ReceiveActorBeginOverlap`
  (params (OtherActor :type "Actor Object Reference"))
  (`parent.ReceiveActorBeginOverlap` null))

(event `self.ReceiveTick`
  (params (DeltaSeconds :type "Float (single-precision)"))
  (`parent.ReceiveTick` DeltaSeconds))

(event `ToggleLaser`
  (params (`Toggle A` :type Boolean) (`Toggle B` :type Boolean))
  (bind _laseractor (`self.LaserActor`))
  (`/Engine/EditorBlueprintResources/StandardMacros.FlipFlop`
    (:`A`
      (set `self.LaserShow?` false)
      (bind _output_get (set `self.LaserShow?` `Toggle A`))
      (`SceneComponent.SetVisibility` _laseractor _output_get false))
    (:`B`
      (set `self.LaserShow?` false)
      (bind _output_get_2 (set `self.LaserShow?` `Toggle B`))
      (`SceneComponent.SetVisibility` _laseractor _output_get_2 false))))

(event `StartShooting`
  (bind _returnvalue (`KismetSystemLibrary.K2_SetTimerDelegate` (delegate `Shoot`) 0.1 true -0.1)))

(event `StopShooting`
  (`KismetSystemLibrary.K2_ClearAndInvalidateTimerHandle` (stale `StartShooting` _returnvalue))
  (`PlayerCameraManager.StopCameraShake` (`GameplayStatics.GetPlayerCameraManager` 0) null false))

(event `Shoot`
  (bind _muzzleflashlocation (`self.MuzzleFlashLocation`))
  (bind (_worldlocation _worlddirection) (`PlayerController.DeprojectMousePositionToWorld` (`GameplayStatics.GetPlayerController` 0)))
  (bind _returnvalue (`NiagaraFunctionLibrary.SpawnSystemAttached` "/Game/sA_Megapack_v1/sA_ShootingVfxPack/FX/NiagaraSystems/NS_AR_Muzzleflash_1_ONCE.NS_AR_Muzzleflash_1_ONCE" _muzzleflashlocation "None" (`SceneComponent.K2_GetComponentLocation` _muzzleflashlocation) (`SceneComponent.K2_GetComponentRotation` _muzzleflashlocation) "KeepWorldPosition"))
  (`SceneComponent.SetWorldScale3D` _returnvalue (4.0 4.0 4.0))
  (`GameplayStatics.PlaySoundAtLocation` null (`self.K2_GetActorLocation`) (struct) 1.0 1.0 0.0 null null null null)
  (bind _outhit (`KismetSystemLibrary.LineTraceSingle` _worldlocation (+ _worldlocation (* _worlddirection 10000.0)) "TraceTypeQuery2" true))
  (bind (_bblockinghit _binitialoverlap _time _distance _location _impactpoint _normal _impactnormal _physmat _hitactor _hitcomponent _hitbonename _bonename _hititem _elementindex _faceindex _tracestart) (`GameplayStatics.BreakHitResult` _outhit))
  (`GameplayStatics.ApplyPointDamage` _hitactor (`self.WeaponDamage`) _tracestart _outhit null self))

(fn `UserConstructionScript`
  (`parent.UserConstructionScript`))