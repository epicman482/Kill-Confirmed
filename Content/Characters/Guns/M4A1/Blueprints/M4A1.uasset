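; M4A1 gun Blueprint, a child class that adds a switchable laser to the behavior it inherits.
; BeginPlay, ActorBeginOverlap, Tick and the construction script only forward to the parent.
; A ToggleLaser event uses a FlipFlop to alternate between its two caller-supplied booleans, applying each as the visibility of LaserActor without propagating to children.
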(event `self.ReceiveBeginPlay`
  (`parent.ReceiveBeginPlay`))

(event `self.ReceiveActorBeginOverlap`
  (params (OtherActor :type "Actor Object Reference"))
  (`parent.ReceiveActorBeginOverlap` null))

(event `self.ReceiveTick`
  (params (DeltaSeconds :type "Float (single-precision)"))
  (`parent.ReceiveTick` DeltaSeconds))

(event `ToggleLaser`
  (params (`Toggle A` :type Boolean) (`Toggle B` :type Boolean))
  (bind _laseractor (`self.LaserActor`))
  (`/Engine/EditorBlueprintResources/StandardMacros.FlipFlop`
    (:`A`
      (`SceneComponent.SetVisibility` _laseractor `Toggle A` false))
    (:`B`
      (`SceneComponent.SetVisibility` _laseractor `Toggle B` false))))

(fn `UserConstructionScript`
  (`parent.UserConstructionScript`))